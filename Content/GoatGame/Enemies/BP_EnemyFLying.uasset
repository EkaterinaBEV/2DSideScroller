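; BP_EnemyFLying is a flying enemy that shoots at the goat and is destroyed by any damage.
; A looping-style flapping sound is attached on BeginPlay and stopped when the enemy is damaged or destroyed.
; When BP_Goat begins overlapping the Sphere, it spawns one scaled-down BP_EnemyProj at the Scene component, rotated toward the player pawn, with a lightning sound.
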(event OnComponentBeginOverlap(Sphere)
  (params (OverlappedComponent :type Primitive%20Component%20Object%20Reference) (OtherActor :type Actor%20Object%20Reference) (OtherComp :type Primitive%20Component%20Object%20Reference) (OtherBodyIndex :type Integer) (bFromSweep :type Boolean) (SweepResult :type Hit%20Result%20Structure%20%28by%20ref%29))
  (bind _returnvalue (Transformation|GetActorLocation))
  (bind _returnvalue_2 (Game|Player|GetPlayerPawn 0))
  (bind _scene (Variables|Default|GetScene))
  (bind _returnvalue_3 (Transformation|GetWorldLocation _scene))
  (bind _returnvalue_4 (Transformation|GetActorLocation _returnvalue_2))
  (bind _returnvalue_5 (Math|Rotator|FindLookatRotation _returnvalue _returnvalue_4))
  (Utilities|Casting|CastToBP_Goat OtherActor)
  (Game|SpawnActorfromClass "/Game/GoatGame/Enemies/Projectile/BP_EnemyProj.BP_EnemyProj_C" (Math|Transform|MakeTransform _returnvalue_3 _returnvalue_5 "0.200000,0.200000,0.200000") "Undefined" 0 0)
  (Audio|PlaySoundatLocation "/Game/GoatGame/SOunds/S_Lightning.S_Lightning" _returnvalue_3 _returnvalue_5 1.0 1.0 0.0 0 0 0 0))

(event EventBeginPlay
  (bind _returnvalue (Audio|SpawnSoundAttached "/Game/GoatGame/SOunds/S_Flapping.S_Flapping" (Variables|Default|GetScene) "None" "0, 0, 0" "0, 0, 0" "KeepRelativeOffset" false 1.0 1.0 0.0 0 0))
  (Variables|Default|SetSoundFlying _returnvalue))

(event EventDestroyed
  (bind _soundflying (Variables|Default|GetSoundFlying))
  (Utilities|IsValid _soundflying
    (:Is%20Valid
      (Audio|Components|Audio|Stop _soundflying))))

(event Game|Damage|EventAnyDamage
  (params (Damage :type Float%20%28single-precision%29) (DamageType :type Damage%20Type%20Object%20Reference) (InstigatedBy :type Controller%20Object%20Reference) (DamageCauser :type Actor%20Object%20Reference))
  (bind _soundflying (Variables|Default|GetSoundFlying))
  (Actor|DestroyActor)
  (Utilities|IsValid _soundflying
    (:Is%20Valid
      (Audio|Components|Audio|Stop _soundflying))))

(fn ConstructionScript)