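; BP_Enemy is a flipbook-based enemy that hurts the goat on contact and dies to any damage.
; On BeginPlay it attaches a looping-style walk sound to its flipbook and keeps a reference to it.
; Its Box overlap casts to BP_Goat and calls WhenHit with its Damage value.
; Any damage destroys the actor, and both that path and Destroyed stop the walk sound.
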(event OnComponentBeginOverlap(Box)
  (params (OverlappedComponent :type Primitive%20Component%20Object%20Reference) (OtherActor :type Actor%20Object%20Reference) (OtherComp :type Primitive%20Component%20Object%20Reference) (OtherBodyIndex :type Integer) (bFromSweep :type Boolean) (SweepResult :type Hit%20Result%20Structure%20%28by%20ref%29))
  (bind _asbp_goat (Utilities|Casting|CastToBP_Goat OtherActor))
  (Default|WhenHit _asbp_goat (Variables|Default|GetDamage)))

(event EventBeginPlay
  (bind _returnvalue (Audio|SpawnSoundAttached "/Game/GoatGame/SOunds/S_Walk.S_Walk" (Variables|Default|GetPaperFlipbook) "None" "0, 0, 0" "0, 0, 0" "KeepRelativeOffset" false 1.0 1.0 0.0 0 0))
  (Variables|Default|SetSound _returnvalue))

(event EventDestroyed
  (bind _sound (Variables|Default|GetSound))
  (Utilities|IsValid _sound
    (:Is%20Valid
      (Audio|Components|Audio|Stop _sound))))

(event Game|Damage|EventAnyDamage
  (params (Damage :type Float%20%28single-precision%29) (DamageType :type Damage%20Type%20Object%20Reference) (InstigatedBy :type Controller%20Object%20Reference) (DamageCauser :type Actor%20Object%20Reference))
  (bind _sound (Variables|Default|GetSound))
  (Actor|DestroyActor)
  (Utilities|IsValid _sound
    (:Is%20Valid
      (Audio|Components|Audio|Stop _sound))))

(fn ConstructionScript)