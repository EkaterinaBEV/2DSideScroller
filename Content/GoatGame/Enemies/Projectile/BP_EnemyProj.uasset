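; BP_EnemyProj is an enemy projectile that damages goats on contact.
; Its sphere overlap event applies damage to actors tagged Goat, crediting the projectile's owner, then destroys the projectile.
; An overlap with an actor tagged Proj destroys both actors, while other valid actors are ignored.
; An invalid overlapping actor leads to self-destruction after a short delay.
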(event OnComponentBeginOverlap(Sphere)
  (params (OverlappedComponent :type Primitive%20Component%20Object%20Reference) (OtherActor :type Actor%20Object%20Reference) (OtherComp :type Primitive%20Component%20Object%20Reference) (OtherBodyIndex :type Integer) (bFromSweep :type Boolean) (SweepResult :type Hit%20Result%20Structure%20%28by%20ref%29))
  (Utilities|IsValid OtherActor
    (:Is%20Valid
      (if (Actor|ActorHasTag OtherActor "Goat")
        (Game|Damage|ApplyDamage OtherActor 1.0 0 (Components|GetOwner))
        (Actor|DestroyActor :!label _label)
        (elif (Actor|ActorHasTag OtherActor "Proj")
          (Utilities|IsValid OtherActor
            (:Is%20Valid
              (Actor|DestroyActor OtherActor)
              (Actor|DestroyActor))))))
    (:Is%20Not%20Valid
      (Utilities|FlowControl|Delay 0.5)
      (goto _label))))

(event EventBeginPlay)

(event Collision|EventActorBeginOverlap
  (params (OtherActor :type Actor%20Object%20Reference)))

(event EventTick
  (params (DeltaSeconds :type Float%20%28single-precision%29)))

(fn ConstructionScript)