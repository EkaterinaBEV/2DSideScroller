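; BP_Flower is a flower enemy in the goat game that hurts the player goat on contact.
; Its Box overlap casts the other actor to BP_Goat and calls WhenHit with the flower's Damage.
; On BeginPlay it plays S_Ding attached to its PaperSprite, keeping the audio component so it can stop the sound when the flower is destroyed.
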(event OnComponentBeginOverlap(Box)
  (params (OverlappedComponent :type Primitive%20Component%20Object%20Reference) (OtherActor :type Actor%20Object%20Reference) (OtherComp :type Primitive%20Component%20Object%20Reference) (OtherBodyIndex :type Integer) (bFromSweep :type Boolean) (SweepResult :type Hit%20Result%20Structure%20%28by%20ref%29))
  (bind _asbp_goat (Utilities|Casting|CastToBP_Goat OtherActor))
  (Default|WhenHit _asbp_goat (Variables|Default|GetDamage)))

(event EventBeginPlay
  (bind _returnvalue (Audio|SpawnSoundAttached "/Game/GoatGame/SOunds/S_Ding.S_Ding" (Variables|Default|GetPaperSprite) "None" "0, 0, 0" "0, 0, 0" "KeepRelativeOffset" false 1.0 1.0 0.0 0 0))
  (Variables|Default|SetSoundFlower _returnvalue))

(event Collision|EventActorBeginOverlap
  (params (OtherActor :type Actor%20Object%20Reference)))

(event EventTick
  (params (DeltaSeconds :type Float%20%28single-precision%29)))

(event EventDestroyed
  (bind _soundflower (Variables|Default|GetSoundFlower))
  (Utilities|IsValid _soundflower
    (:Is%20Valid
      (Audio|Components|Audio|Stop _soundflower))))

(fn ConstructionScript)