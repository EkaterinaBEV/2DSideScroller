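; BP_EndlessBase is a floor segment that endlessly extends the level for the goat player.
; When BP_Goat enters the Box trigger, it waits one second, then spawns one of three segment classes at random at its Arrow component, which marks the next attachment point.
; Overlapping the KillZone saves the goat's game, pauses play and shows the EndGame widget with UI-only mouse input.
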(event OnComponentBeginOverlap(Box)
  (params (OverlappedComponent :type Primitive%20Component%20Object%20Reference) (OtherActor :type Actor%20Object%20Reference) (OtherComp :type Primitive%20Component%20Object%20Reference) (OtherBodyIndex :type Integer) (bFromSweep :type Boolean) (SweepResult :type Hit%20Result%20Structure%20%28by%20ref%29))
  (bind _arrow (Variables|Default|GetArrow))
  (bind _arrow_2 (Variables|Default|GetArrow))
  (bind _returnvalue (Transformation|GetWorldTransform _arrow))
  (bind _returnvalue_2 (Transformation|GetWorldTransform _arrow_2))
  (Utilities|Casting|CastToBP_Goat OtherActor)
  (Utilities|FlowControl|Delay 1.0)
  (bind _output_get (Variables|Default|SetInt (Math|Random|RandomIntegerinRange 0 2)))
  (switch int _output_get
    (:0
      (Game|SpawnActorfromClass "BP_EndlessBase_C" (Transformation|GetWorldTransform (Variables|Default|GetArrow)) "Undefined" 0 0))
    (:1
      (Game|SpawnActorfromClass "/Game/GoatGame/FLoor/BP_EndlessBase1.BP_EndlessBase1_C" (Math|Transform|MakeTransform (.location _returnvalue_2) "0, 0, 0" (.scale _returnvalue_2)) "Undefined" 0 0))
    (:2
      (Game|SpawnActorfromClass "/Game/GoatGame/FLoor/BP_EndlessBase2.BP_EndlessBase2_C" (Math|Transform|MakeTransform (.location _returnvalue) "0, 0, 0" (.scale _returnvalue)) "Undefined" 0 0))))

(event OnComponentBeginOverlap(KillZone)
  (params (OverlappedComponent :type Primitive%20Component%20Object%20Reference) (OtherActor :type Actor%20Object%20Reference) (OtherComp :type Primitive%20Component%20Object%20Reference) (OtherBodyIndex :type Integer) (bFromSweep :type Boolean) (SweepResult :type Hit%20Result%20Structure%20%28by%20ref%29))
  (bind _returnvalue (Game|GetPlayerController 0))
  (bind _asbp_goat (Utilities|Casting|CastToBP_Goat OtherActor))
  (Default|GoatSaveGame _asbp_goat)
  (Game|SetGamePaused true)
  (bind _returnvalue_2 (UserInterface|CreateWidget "/Game/GoatGame/HUD/EndGame.EndGame_C"))
  (UserInterface|Viewport|AddtoViewport _returnvalue_2 0)
  (Variables|/Script/Engine.PlayerController|SetbShowMouseCursor _returnvalue true)
  (Input|SetInputModeUIOnly _returnvalue 0 "DoNotLock"))

(event Collision|EventActorBeginOverlap
  (params (OtherActor :type Actor%20Object%20Reference)))

(event EventTick
  (params (DeltaSeconds :type Float%20%28single-precision%29)))

(fn ConstructionScript)